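; Player controller for a city builder that drives a top-down camera and grid-based building placement.
; On BeginPlay it adds the demo UI and input context, spawns the camera, and finds its start, bounds and snap target.
; Input forwards movement, rotation, zoom and snapping to the camera.
; Each tick selects the tile under the cursor and moves a preview actor there; clicking on a valid spot spawns the building and exits placement mode.
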(event Input|EnhancedActionEvents|EnhancedInputActionIA_MoveCameraForward
  (params (ActionValue :type Float%20%28double-precision%29) (ElapsedSeconds :type Float%20%28double-precision%29) (TriggeredSeconds :type Float%20%28double-precision%29) (InputAction :type Input%20Action%20Object%20Reference :default "/Game/Blueprint/Input/IA_MoveCameraForward.IA_MoveCameraForward"))
  ;[0.4029 0 1 0.15 16] Inputs for Moving the camera
  (Default|MoveCameraForward (Variables|Camera|GetTopDownCamera) ActionValue))

(event Input|EnhancedActionEvents|EnhancedInputActionIA_MoveCameraRight
  (params (ActionValue :type Float%20%28double-precision%29) (ElapsedSeconds :type Float%20%28double-precision%29) (TriggeredSeconds :type Float%20%28double-precision%29) (InputAction :type Input%20Action%20Object%20Reference :default "/Game/Blueprint/Input/IA_MoveCameraRight.IA_MoveCameraRight"))
  ;[0.4029 0 1 0.15 16] Inputs for Moving the camera
  (Default|MoveCameraRight (Variables|Camera|GetTopDownCamera) ActionValue))

(event Input|EnhancedActionEvents|EnhancedInputActionIA_RotateCamera
  (params (ActionValue :type Float%20%28double-precision%29) (ElapsedSeconds :type Float%20%28double-precision%29) (TriggeredSeconds :type Float%20%28double-precision%29) (InputAction :type Input%20Action%20Object%20Reference :default "/Game/Blueprint/Input/IA_RotateCamera.IA_RotateCamera"))
  ;[0.4029 0 1 0.15 16] Inputs for Rotating the camera
  (Default|RotateCameraHorizontal (Variables|Camera|GetTopDownCamera) ActionValue))

(event Input|EnhancedActionEvents|EnhancedInputActionIA_MoveCameraUp
  (params (ActionValue :type Float%20%28double-precision%29) (ElapsedSeconds :type Float%20%28double-precision%29) (TriggeredSeconds :type Float%20%28double-precision%29) (InputAction :type Input%20Action%20Object%20Reference :default "/Game/Blueprint/Input/IA_MoveCameraUp.IA_MoveCameraUp"))
  ;[0.4029 0 1 0.15 16] Inputs for Moving the camera
  (Default|MoveCameraUp (Variables|Camera|GetTopDownCamera) ActionValue))

(event Input|EnhancedActionEvents|EnhancedInputActionIA_ZoomCamera
  (params (ActionValue :type Float%20%28double-precision%29) (ElapsedSeconds :type Float%20%28double-precision%29) (TriggeredSeconds :type Float%20%28double-precision%29) (InputAction :type Input%20Action%20Object%20Reference :default "/Game/Blueprint/Input/IA_ZoomCamera.IA_ZoomCamera"))
  ;[0.4029 0 1 0.15 16] Inputs for zooming the camera
  (Default|ZoomCamera (Variables|Camera|GetTopDownCamera) ActionValue))

(event Input|EnhancedActionEvents|EnhancedInputActionIA_MouseClick
  (params (ActionValue :type Boolean) (ElapsedSeconds :type Float%20%28double-precision%29) (TriggeredSeconds :type Float%20%28double-precision%29) (InputAction :type Input%20Action%20Object%20Reference :default "/Game/Blueprint/Input/IA_MouseClick.IA_MouseClick"))
  (if (Variables|Default|GetIsPlacementMoveEnabled)
    (CallFunction|SpawnBuilding)))

(event EventTick
  (params (DeltaSeconds :type Float%20%28single-precision%29))
  (CallFunction|UpdateCursorPosition)
  (if (Variables|Default|GetIsPlacementMoveEnabled)
    (CallFunction|UpdatePlacement)))

(event EventBeginPlay
  (bind _asgm_city_builder (Utilities|Casting|CastToGM_CityBuilder (Game|GetGameMode)))
  (Variables|Default|SetAs%20GM%20City%20Builder _asgm_city_builder)
  (bind _returnvalue (Actor|GetActorOfClass "/Game/Blueprint/CellularAutomata/BP_CA_CityLayout.BP_CA_CityLayout_C"))
  (Variables|Default|SetAs%20BP_CA_City_Layout _returnvalue)
  (CallFunction|SetPlacementModeEnabled true)
  (bind _returnvalue_2 (UserInterface|CreateWidget "/Game/TopDownCamera/Demo/UI/WB_Demo_UI.WB_Demo_UI_C"))
  (UserInterface|Viewport|AddtoViewport _returnvalue_2 0)
  (Input|AddMappingContext (PlayerController|LocalPlayerSubsystems|GetEnhancedInputLocalPlayerSubsystem) "/Game/Blueprint/Input/IMC_PlayerControl.IMC_PlayerControl" 0 "(bIgnoreAllPressedKeysUntilRelease=True,bForceImmediately=False,bNotifyUserSettings=False)")
  ;[0.4029 0 1 0.15 16] Creates a new camera, retrieves its reference, and switches to using this camera.
  (bind _returnvalue_3 (Game|SpawnActorfromClass "/Game/TopDownCamera/Blueprints/BP_TopDownCamera.BP_TopDownCamera_C" (Math|Transform|MakeTransform "0, 0, 0" "0, 0, 0" "1.000000,1.000000,1.000000") "Undefined" "OverrideRootScale" 0 0))
  (bind _output_get (Variables|Camera|SetTopDownCamera _returnvalue_3))
  (Game|Player|SetViewTargetwithBlend _output_get 0.0 "VTBlend_Linear" 0.0 false)
  (Utilities|FlowControl|Sequence
    (:then_0
      ;[0.4029 0 1 0.15 16] Creates a Play Start Actor on the level; the camera will use its values for initial positioning after spawn.
      (bind _returnvalue_4 (Actor|GetActorOfClass "/Script/Engine.PlayerStart"))
      (Utilities|IsValid _returnvalue_4
        (:Is%20Valid
          (Transformation|SetActorLocation (Variables|Camera|GetTopDownCamera) (Transformation|GetActorLocation _returnvalue_4) false false)
          (Default|SetCameraInitialValues (Variables|Camera|GetTopDownCamera) (.pitch (Transformation|GetActorRotation _returnvalue_4)) (.yaw (Transformation|GetActorRotation _returnvalue_4)) 3e+03))))
    (:then_1
      ;[0.4029 0 1 0.15 16] Place the BP_Demo_BlockingArea actor in the level to create a complex area that restricts the camera's movement beyond its boundaries.
      ; Ensure to activate the EnableComplexBlockingArea variable on the camera to enable this functionality.
      (bind _returnvalue_5 (Actor|GetActorOfClass "/Game/TopDownCamera/Demo/BP_Demo_BlockingArea.BP_Demo_BlockingArea_C"))
      (Utilities|IsValid _returnvalue_5
        (:Is%20Valid
          (Default|SetComplexBlockingAreaPoints (Variables|Camera|GetTopDownCamera) (Variables|/Game/TopDownCamera/Demo/BP_Demo_BlockingArea.BP_Demo_BlockingArea_C|GetSplinePoints _returnvalue_5)))))
    (:then_2
      ;[0.4029 0 1 0.15 16] In the demo, actor BP_Demo_Target is used as the target. You can replace it, for example, with your own character.
      (bind _returnvalue_6 (Actor|GetActorOfClass "/Game/TopDownCamera/Demo/BP_Demo_Target.BP_Demo_Target_C"))
      (Utilities|IsValid _returnvalue_6
        (:Is%20Valid
          (Variables|Camera|SetCameraTarget _returnvalue_6))))))

(event Input|MouseEvents|MouseY
  (params (AxisValue :type Float%20%28single-precision%29))
  ;[0.4029 0 1 0.15 16] Inputs for Rotating the camera
  (if (Variables|Camera|GetMMBPressed)
    (Default|RotateCameraVertical (Variables|Camera|GetTopDownCamera) AxisValue)))

(event Input|MouseEvents|MouseX
  (params (AxisValue :type Float%20%28single-precision%29))
  ;[0.4029 0 1 0.15 16] Inputs for Rotating the camera
  (if (Variables|Camera|GetMMBPressed)
    (Default|RotateCameraHorizontal (Variables|Camera|GetTopDownCamera) AxisValue)))

(event Input|KeyboardEvents|R
  (params (Key :type Key%20Structure :default "None"))
  ;[0.4029 0 1 0.15 16] Inputs for Rotating the camera
  (:Pressed
    (Default|RotateCameratoFixedAngle (Variables|Camera|GetTopDownCamera) 9e+01)))

(event Input|KeyboardEvents|T
  (params (Key :type Key%20Structure :default "None"))
  ;[0.4029 0 1 0.15 16] Inputs for Rotating the camera
  (:Pressed
    (Default|RotateCameratoFixedAngle (Variables|Camera|GetTopDownCamera) -9e+01)))

(event Input|MouseEvents|MiddleMouseButton
  (params (Key :type Key%20Structure :default "None"))
  ;[0.4029 0 1 0.15 16] Inputs for Rotating the camera
  (:Pressed
    (Variables|Camera|SetMMBPressed true))
  (:Released
    (Variables|Camera|SetMMBPressed false)))

(event Input|KeyboardEvents|LeftShift
  (params (Key :type Key%20Structure :default "None"))
  (bind _topdowncamera (Variables|Camera|GetTopDownCamera))
  ;[0.4029 0 1 0.15 16] Inputs for Moving the camera
  (:Pressed
    (Default|ActivateBoostonMove _topdowncamera true))
  (:Released
    (Default|ActivateBoostonMove _topdowncamera false)))

(event Input|KeyboardEvents|F
  (params (Key :type Key%20Structure :default "None"))
  (bind _topdowncamera (Variables|Camera|GetTopDownCamera))
  ;[0.4029 0 1 0.15 16] Inputs for snapping the camera to the target.
  (:Pressed
    (if (Default|IsCameraSnappingtoTarget (Variables|Camera|GetTopDownCamera))
      (Default|UnsnapCamerafromTarget _topdowncamera)
      (else
        (Default|SnapCameratoTarget _topdowncamera (Variables|Camera|GetCameraTarget))))))

(event Input|KeyboardEvents|SpaceBar
  (params (Key :type Key%20Structure :default "None"))
  (bind _hitresult (Game|Player|GetHitResultUnderCursorbyChannel "TraceTypeQuery1" true))
  (bind (_bblockinghit _binitialoverlap _time _distance _location) (Collision|BreakHitResult _hitresult))
  ;[0.4029 0 1 0.15 16] Inputs for snapping the camera to the target.
  (:Pressed
    (if _bblockinghit
      (Default|MoveCameratoLocation (Variables|Camera|GetTopDownCamera) _location))))

(event Input|KeyboardEvents|1
  (params (Key :type Key%20Structure :default "None"))
  (:Pressed
    (CallFunction|SetPlacementModeEnabled true)))

(event Input|KeyboardEvents|0
  (params (Key :type Key%20Structure :default "None"))
  (bind _as_bp_ca_city_layout (Variables|Default|GetAs%20BP_CA_City_Layout))
  (bind _instancedgridmesh (Variables|/Script/MLCA_CityGenerator.CA_CityLayout|GetInstancedGridMesh _as_bp_ca_city_layout))
  (:Pressed
    (for _index (range 0 (- (Components|InstancedStaticMesh|GetInstanceCount _instancedgridmesh) 1))
      (Components|InstancedStaticMesh|SetCustomDataValue _instancedgridmesh _index 0 0.0 false)
      (Components|InstancedStaticMesh|SetCustomDataValue _instancedgridmesh _index 1 0.0 false)
      (Components|InstancedStaticMesh|SetCustomDataValue _instancedgridmesh _index 2 0.0 false))))

(fn ConstructionScript)

(fn SetPlacementModeEnabled
  (params (IsEnabled :type Boolean))
  (if (== IsEnabled (Variables|Default|GetIsPlacementMoveEnabled))
    (return)
    (else
      (bind _output_get (Variables|Default|SetIsPlacementMoveEnabled IsEnabled))
      (if _output_get
        (bind _returnvalue (Game|SpawnActorfromClass (Variables|Default|GetPlaceableActorType) (Math|Transform|MakeTransform "0.000000,0.000000,-100000.000000" "0, 0, 0" "1.000000,1.000000,1.000000") "AlwaysSpawn" "MultiplyWithRoot" 0 0))
        (bind _output_get_2 (Variables|Default|SetPlaceableActor _returnvalue))
        (Utilities|IsValid (Actor|GetComponentbyClass _output_get_2 "/Game/Blueprint/Components/BPC_ClickableComponent.BPC_ClickableComponent_C")
          (:Is%20Valid
            (Default|InPlacementMode (Actor|GetComponentbyClass _output_get_2 "/Game/Blueprint/Components/BPC_ClickableComponent.BPC_ClickableComponent_C")))
          (:Is%20Not%20Valid
            _))
        (AddComponent|AddBPCSpawnable _output_get_2)
        (else
          (Utilities|IsValid (Variables|Default|GetPlaceableActor)
            (:Is%20Valid
              (Actor|DestroyActor (Variables|Default|GetPlaceableActor)))))))))

(fn UpdatePlacement
  (bind _placeableactor (Variables|Default|GetPlaceableActor))
  (bind _as_gm_city_builder (Variables|Default|GetAs%20GM%20City%20Builder))
  (bind _gridref (Default|GetGrid _as_gm_city_builder))
  (if (Variables|/Game/Blueprint/Grid/BP_Grid.BP_Grid_C|GetIsValidTile? _gridref)
    (Rendering|SetActorHiddenInGame _placeableactor false)
    (Transformation|SetActorLocation _placeableactor (Variables|/Game/Blueprint/Grid/BP_Grid.BP_Grid_C|GetSelectedTileLocation _gridref) true false)
    (else
      (Rendering|SetActorHiddenInGame _placeableactor true))))

(fn SpawnBuilding
  (bind _placeableactor (Variables|Default|GetPlaceableActor))
  (bind _returnvalue (Actor|GetComponentbyClass _placeableactor "/Game/Blueprint/Components/BPC_Spawnable.BPC_Spawnable_C"))
  (Utilities|IsValid _returnvalue
    (:Is%20Valid
      (if (and (Variables|/Game/Blueprint/Components/BPC_Spawnable.BPC_Spawnable_C|GetIsPlacementValid _returnvalue) (Variables|/Game/Blueprint/Grid/BP_Grid.BP_Grid_C|GetIsValidTile? (Default|GetGrid (Variables|Default|GetAs%20GM%20City%20Builder))))
        (Game|SpawnActorfromClass (Variables|Default|GetPlaceableActorType) (Transformation|GetActorTransform (Variables|Default|GetPlaceableActor)) "AlwaysSpawn" "MultiplyWithRoot" 0 0)
        (CallFunction|SetPlacementModeEnabled false)))))

(fn UpdateCursorPosition
  (bind _returnvalue (Game|GetPlayerController 0))
  (bind (_hitresult _returnvalue_2) (Game|Player|GetHitResultUnderCursorbyChannel _returnvalue "TraceTypeQuery1" true))
  (LocalVariables|SetGrid (Default|GetGrid (Variables|Default|GetAs%20GM%20City%20Builder)))
  (if _returnvalue_2
    (LocalVariables|SetHitLocation (.Location (Collision|BreakHitResult _hitresult)))
    (bind (_isvalid_ _row _column) (Default|LocationtoTile (LocalVariables|GetGrid) (LocalVariables|GetHitLocation)))
    (Default|SetSelectedTile (LocalVariables|GetGrid) _row _column)
    (else
      (Default|SetSelectedTile (LocalVariables|GetGrid) -1 -1))))