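; Procedural terrain actor that builds a noise-driven height grid mesh with collision; despite the DiamondSquare name, its heights come from FastNoise.
; The construction script configures the noise, then CreateVertices fills scaled positions and UVs and CreateTriangles indexes two triangles per cell.
; It computes normals and tangents before creating the mesh section and applying the material.
; BeginPlay is empty, its old build chain is disconnected, and CreateVertex and CreateTriangle are unused.
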(event EventBeginPlay)

(fn ConstructionScript
  (bind _returnvalue (Game|ConstructObjectfromClass "/Script/FastNoiseGenerator.FastNoiseWrapper"))
  (bind _output_get (Variables|Default|SetNoise _returnvalue))
  (Class|FastNoiseWrapper|SetupFastNoise _output_get (Variables|Default|GetNoise%20Type) (Variables|Default|GetSeed) (Variables|Default|GetFrequency) (Variables|Default|GetInterp) (Variables|Default|GetFractaltype) (Variables|Default|GetOctaves) (Variables|Default|GetLacunarity) (Variables|Default|GetGain) (Variables|Default|GetCellular%20Jitter) (Variables|Default|GetCellular%20Distance%20Function) (Variables|Default|GetCellular%20Return%20Type))
  (Utilities|Array|Clear (Variables|Default|GetVertices))
  (Utilities|Array|Clear (Variables|Default|GetTriangles))
  (CallFunction|CreateVertices)
  (CallFunction|CreateTriangles)
  (bind (_normals _tangents) (Class|KismetProceduralMeshLibrary|CalculateTangentsforMesh (Variables|Default|GetVertices) (Variables|Default|GetTriangles) (Variables|Default|GetUV0)))
  (Variables|Default|SetNormals _normals)
  (Variables|Default|SetTangents _tangents)
  (Class|ProceduralMeshComponent|CreateMeshSectionLinearColor (Variables|Default|GetProceduralMesh) 0 (Variables|Default|GetVertices) (Variables|Default|GetTriangles) (Variables|Default|GetNormals) (Variables|Default|GetUV0) 0 0 0 0 (Variables|Default|GetTangents) true false)
  (Rendering|Material|SetMaterial (Variables|Default|GetProceduralMesh) 0 (Variables|Default|GetMaterial)))

(fn CreateVertices
  (for _index (range 0 (Variables|Default|GetXSize))
    (LocalVariables|SetX _index)
    (for _index_2 (range 0 (Variables|Default|GetYSize))
      (LocalVariables|SetY _index_2)
      (Utilities|Array|Add (Variables|Default|GetVertices) (Math|Vector|MakeVector (* (Variables|Default|GetScale) (LocalVariables|GetX)) (* (Variables|Default|GetScale) (LocalVariables|GetY)) (* (Class|FastNoiseWrapper|GetNoise2D (Variables|Default|GetNoise) (Math|Conversions|ToFloat(Integer) (LocalVariables|GetX)) (Math|Conversions|ToFloat(Integer) (LocalVariables|GetY))) (Variables|Default|GetZMultiplier))))
      (Utilities|Array|Add (Variables|Default|GetUV0) (Math|Vector2D|MakeVector2D (* (Variables|Default|GetUVScale) (LocalVariables|GetX)) (* (Variables|Default|GetUVScale) (LocalVariables|GetY)))))))

(fn CreateTriangles
  (for _index (range 0 (- (Variables|Default|GetXSize) 1))
    (for _index_2 (range 0 (- (Variables|Default|GetYSize) 1))
      (Utilities|Array|Add (Variables|Default|GetTriangles) (LocalVariables|GetVertex))
      (Utilities|Array|Add (Variables|Default|GetTriangles) (+ (LocalVariables|GetVertex) 1))
      (Utilities|Array|Add (Variables|Default|GetTriangles) (+ (Variables|Default|GetYSize) 1 (LocalVariables|GetVertex)))
      (Utilities|Array|Add (Variables|Default|GetTriangles) (+ (LocalVariables|GetVertex) 1))
      (Utilities|Array|Add (Variables|Default|GetTriangles) (+ (Variables|Default|GetYSize) 2 (LocalVariables|GetVertex)))
      (Utilities|Array|Add (Variables|Default|GetTriangles) (+ (Variables|Default|GetYSize) 1 (LocalVariables|GetVertex)))
      (Math|Integer|IncrementInt (LocalVariables|GetVertex)))
    (Math|Integer|IncrementInt (LocalVariables|GetVertex))))

(fn CreateVertex
  (params (X :type Integer) (Y :type Integer))
  (Utilities|Array|Add (Variables|Default|GetVertices) (Math|Vector|MakeVector (* (Variables|Default|GetScale) X) (* (Variables|Default|GetScale) Y) 0.0))
  (Utilities|Array|Add (Variables|Default|GetUV0) (Math|Vector2D|MakeVector2D (* (Variables|Default|GetUVScale) X) (* (Variables|Default|GetUVScale) Y))))

(fn CreateTriangle
  (params (Vertex :type Integer%20%28by%20ref%29))
  (Utilities|Array|Add (Variables|Default|GetTriangles) Vertex)
  (Utilities|Array|Add (Variables|Default|GetTriangles) (+ Vertex 1))
  (Utilities|Array|Add (Variables|Default|GetTriangles) (+ (Variables|Default|GetYSize) 1 Vertex))
  (Utilities|Array|Add (Variables|Default|GetTriangles) (+ Vertex 1))
  (Utilities|Array|Add (Variables|Default|GetTriangles) (+ (Variables|Default|GetYSize) 2 Vertex))
  (Utilities|Array|Add (Variables|Default|GetTriangles) (+ (Variables|Default|GetYSize) 1 Vertex))
  (Math|Integer|IncrementInt Vertex))