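; BP_EnemyCamp is an enemy camp that spawns a small group of combat enemies and tracks when it has been cleared.
; On BeginPlay it spawns a random number of BP_CombatEnemy actors at random positive X/Y offsets, slightly raised, and binds to each death event.
; Each death decrements the count; the last one sets IsClear, deactivates the fire effect and notifies SpiderManGameMode through CampClearedEvent.
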(event Custom|Handle%20Enemy%20Died
  (bind _result (Math|Integer|DecrementInt (Variables|Default|GetEnemy%20Amount))
    (:%20%20
      (if (<= _result 0)
        (Variables|Default|SetIsClear true)
        (Components|Activation|Deactivate (Variables|Default|GetNS_Fire_Floor_02))
        (Default|CampClearedEvent (Variables|Default|GetAs%20Spider%20Man%20Game%20Mode))))))

(event EventBeginPlay
  (bind _returnvalue (Math|Random|RandomIntegerinRange 100 300))
  (bind _asspider_man_game_mode (Utilities|Casting|CastToSpiderManGameMode (Game|GetGameMode)))
  (Variables|Default|SetAs%20Spider%20Man%20Game%20Mode _asspider_man_game_mode)
  (Variables|Default|SetEnemy%20Amount (Math|Random|RandomIntegerinRange 2 4))
  (for _index (range 1 (Variables|Default|GetEnemy%20Amount))
    (bind _returnvalue_2 (Game|SpawnActorfromClass "/Game/Variant_Combat/Blueprints/AI/BP_CombatEnemy.BP_CombatEnemy_C" (Math|Transform|MakeTransform (+ (+ (Transformation|GetActorLocation) (Math|Vector|MakeVector (Math|Conversions|ToFloat(Integer) _returnvalue) (Math|Conversions|ToFloat(Integer) _returnvalue) 0.0)) "0.000000,0.000000,100.000000") "0, 0, 0" "1.000000,1.000000,1.000000") "AdjustIfPossibleButAlwaysSpawn" "MultiplyWithRoot" 0 0))
    (bind _output_get (Variables|Default|SetNewVar _returnvalue_2))
    (EventDispatchers|BindEventtoOnEnemyDied _output_get (delegate Custom|Handle%20Enemy%20Died))))

(fn ConstructionScript)