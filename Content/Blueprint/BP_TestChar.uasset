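; BP_TestChar is a test Blueprint that rotates its mesh according to the difference between a goal value and a player value.
; The A and D keys raise and lower PlayerLocation by one and print the result.
; Each press then normalizes GoalLocation minus PlayerLocation over a 360-unit range and uses it as the alpha of a shortest-path rotator lerp toward a half turn, setting the mesh's world rotation.
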(event EventBeginPlay)

(event Collision|EventActorBeginOverlap
  (params (OtherActor :type Actor%20Object%20Reference)))

(event EventTick
  (params (DeltaSeconds :type Float%20%28single-precision%29)))

(event Input|KeyboardEvents|A
  (params (Key :type Key%20Structure :default "None"))
  (bind _playerlocation (Variables|Default|GetPlayerLocation))
  (:Pressed
    (Math|Float|IncrementFloat _playerlocation
      (:%20%20
        (Development|PrintString (Utilities|String|ToString(Float) _playerlocation))
        (Transformation|SetWorldRotation (Variables|Character|GetMesh) (Math|Rotator|Lerp(Rotator) "0, 0, 0" "0.000000,180.000000,0.000000" (Math|Float|NormalizetoRange (- (Variables|Default|GetGoalLocation) (Variables|Default|GetPlayerLocation)) 0.0 3.6e+02) true) false false)))))

(event Input|KeyboardEvents|D
  (params (Key :type Key%20Structure :default "None"))
  (bind _playerlocation (Variables|Default|GetPlayerLocation))
  (:Pressed
    (Math|Float|DecrementFloat _playerlocation
      (:%20%20
        (Development|PrintString (Utilities|String|ToString(Float) _playerlocation))
        (Transformation|SetWorldRotation (Variables|Character|GetMesh) (Math|Rotator|Lerp(Rotator) "0, 0, 0" "0.000000,180.000000,0.000000" (Math|Float|NormalizetoRange (- (Variables|Default|GetGoalLocation) (Variables|Default|GetPlayerLocation)) 0.0 3.6e+02) true) false false)))))

(fn ConstructionScript)