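; Generates a procedural city layout from a cellular automata grid on BeginPlay or GenerateMap, clearing previous results and printing the generation time.
; The pipeline simulates and widens roads, extracts districts and sorted roads, assigns district types, then floor-plans them into rectangular blocks.
; Each block spawns a BP_BuildingPCG sized to it, with random height by residential, commercial or industrial type.
; Tree, tile and road-type passes finish the layout.
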(event EventBeginPlay
  (CallFunction|ClearMap)
  (Variables|Default|SetInSeed (Math|Random|RandomInteger 10000))
  (Variables|Default|SetTime (Math|DateTime|Now))
  (Utilities|FlowControl|Sequence
    (:then_0
      (Class|CACityLayout|Initialize)
      (Class|CACityLayout|Simulate)
      (Class|CACityLayout|TrimRoads)
      (Class|CACityLayout|AddRoadWidth)
      (Class|CACityLayout|VisualizeGrid))
    (:then_4
      (Class|CACityLayout|GetAllDistricts)
      (Class|CACityLayout|GetAllRoads)
      (Class|CACityLayout|SelectionSorttheRoad))
    (:then_8
      (Class|CACityLayout|InitializeLayerValues)
      (Class|CACityLayout|CalculateDistrictType)
      (Class|CACityLayout|FloorPlanAllDistricts))
    (:then_12
      (Class|CACityLayout|GetAllLargestRectanglesforDistricts))
    (:then_14
      (CallFunction|AddPCGBuildings))
    (:then_15
      (Class|CACityLayout|SetTreeLayerGridValues)
      (Class|CACityLayout|CalculateTileLayerGridValues)
      (Class|CACityLayout|CalculateRoadType))
    (:then_16
      (Development|PrintString (Utilities|String|Append "City Layout Generation Time :" (Utilities|String|ToString(Float) (Class|KismetMathLibrary|GetTotalMilliseconds (- (Math|DateTime|Now) (Variables|Default|GetTime)))) "ms")))))

(fn ConstructionScript)

(fn GetAllRoad
  (params (RoadArray :type Array%20of%20Road%20Struct%20Structures))
  (bind _output_get (LocalVariables|SetTempGrid (Variables|Default|GetGrid)))
  (for (_array_element _array_index) _output_get
    (if (== _array_element 0)
      (Utilities|Array|Add (LocalVariables|GetNeighborIndex) _array_index)
      (for _array_element_2 (LocalVariables|GetNeighborIndex) :!label _label
        (if (== (Utilities|Array|Get(acopy) (LocalVariables|GetTempGrid) _array_element_2) -2)
          (Utilities|Array|RemoveItem (LocalVariables|GetNeighborIndex) _array_element_2)
          (else
            (CallFunction|RecursivetoRoads (LocalVariables|GetTempGrid) _array_element_2 (LocalVariables|GetTempRoadIndex) (LocalVariables|GetNeighborIndex) (Variables|Default|GetIsMeetJunction))))
        (if (Utilities|Array|IsNotEmpty (LocalVariables|GetNeighborIndex))
          (goto _label)
          (else
            (CallFunction|AddRoadtoArray (LocalVariables|GetTempRoadIndex))))))))

(fn RecursivetoRoads
  (params (GridArray :type Array%20of%20Integers) (Index :type Integer) (RoadIndexArray :type Array%20of%20Integers) (NeighborIndex :type Array%20of%20Integers) (IsMeetJunction :type Boolean))
  (Variables|Default|SetIsMeetJunction false)
  (Utilities|Array|SetArrayElem GridArray Index -3)
  (Utilities|Array|AddUnique RoadIndexArray Index)
  (Utilities|Array|RemoveItem NeighborIndex Index)
  (Utilities|Array|Clear (LocalVariables|GetTempNeighbor))
  (for _array_element (Class|CACityLayout|GetMooreNeighbors (Math|Integer|%(Integer) Index (Variables|Default|GetGridSize)) (/ Index (Variables|Default|GetGridSize)))
    (if (== (Utilities|Array|Get(acopy) GridArray (+ (.X (Utilities|Struct|BreakIntPoint _array_element)) (* (.Y (Utilities|Struct|BreakIntPoint _array_element)) (Variables|Default|GetGridSize)))) 0)
      (Utilities|Array|Add (LocalVariables|GetTempNeighbor) (+ (.X (Utilities|Struct|BreakIntPoint _array_element)) (* (.Y (Utilities|Struct|BreakIntPoint _array_element)) (Variables|Default|GetGridSize))))
      (elif (== (Utilities|Array|Get(acopy) GridArray (+ (.X (Utilities|Struct|BreakIntPoint _array_element)) (* (.Y (Utilities|Struct|BreakIntPoint _array_element)) (Variables|Default|GetGridSize)))) -2)
        (Variables|Default|SetIsMeetJunction true)
        (Utilities|Array|Add NeighborIndex (+ (.X (Utilities|Struct|BreakIntPoint _array_element)) (* (.Y (Utilities|Struct|BreakIntPoint _array_element)) (Variables|Default|GetGridSize))))
        (Utilities|Array|AddUnique RoadIndexArray (+ (.X (Utilities|Struct|BreakIntPoint _array_element)) (* (.Y (Utilities|Struct|BreakIntPoint _array_element)) (Variables|Default|GetGridSize)))))))
  ;[0.15 0.15 0.15 0.5] If meet Junction add valid neighbor
  (if (Variables|Default|GetIsMeetJunction)
    (for _array_element_2 (LocalVariables|GetTempNeighbor)
      (if (Math|Boolean|ORBoolean (== _array_element_2 (- Index 1)) (== _array_element_2 (+ Index 1)) (== _array_element_2 (+ Index (Variables|Default|GetGridSize))) (== _array_element_2 (- Index (Variables|Default|GetGridSize))))
        (Utilities|Array|Add NeighborIndex _array_element_2)))
    (else
      (for _array_element_3 (LocalVariables|GetTempNeighbor)
        (Utilities|Array|Add NeighborIndex _array_element_3)))))

(fn AddRoadtoArray
  (params (RoadIndexArray :type Array%20of%20Integers))
  (for _array_element RoadIndexArray
    (Utilities|Array|Add (LocalVariables|GetArrayLocation) (.location (.OutInstanceTransform (Components|InstancedStaticMesh|GetInstanceTransform (Variables|Default|GetInstancedGridMesh) _array_element false)))))
  (Utilities|Array|Add (Variables|Default|GetRoadArray) (Utilities|Struct|MakeRoadStruct (LocalVariables|GetArrayLocation) RoadIndexArray))
  (Utilities|Array|Clear RoadIndexArray))

(fn AddBuildingBlockISM
  (for _index (range 0 (- (Variables|Default|GetGridSize) 1))
    (for _index_2 (range 0 (- (Variables|Default|GetGridSize) 1))
      (bind _returnvalue (Components|InstancedStaticMesh|AddInstance (Variables|Default|GetISM_BuildingBlocks) (Math|Transform|MakeTransform (Math|Vector|MakeVector (* _index (Variables|Default|GetCellSize)) (* _index_2 (Variables|Default|GetCellSize)) 0.0) "0, 0, 0" "1.000000,1.000000,1.000000") false))
      (Components|InstancedStaticMesh|SetCustomDataValue (Variables|Default|GetISM_BuildingBlocks) _returnvalue 0 0.0 false)
      (Components|InstancedStaticMesh|SetCustomDataValue (Variables|Default|GetISM_BuildingBlocks) _returnvalue 1 0.0 false)
      (Components|InstancedStaticMesh|SetCustomDataValue (Variables|Default|GetISM_BuildingBlocks) _returnvalue 2 0.0 false)
      (Components|InstancedStaticMesh|SetCustomDataValue (Variables|Default|GetISM_BuildingBlocks) _returnvalue 3 0.0 false)
      (Components|InstancedStaticMesh|SetCustomDataValue (Variables|Default|GetISM_BuildingBlocks) _returnvalue 4 0.5 false))))

(fn AddColorISMBuildingBlocks
  (for _array_element (Variables|Default|GetDistrictArray)
    (for _array_element_2 (.BlockCellArray (Utilities|Struct|BreakDistrictStruct _array_element))
      (LocalVariables|SetColor (Math|Color|MakeColor (Math|Random|RandomFloatinRange 0.0 1.0) (Math|Random|RandomFloatinRange 0.0 1.0) (Math|Random|RandomFloatinRange 0.0 1.0)))
      (for _array_element_3 (.BlockArray (Utilities|Struct|BreakBlockCellStruct _array_element_2))
        (Components|InstancedStaticMesh|SetCustomDataValue (Variables|Default|GetISM_BuildingBlocks) _array_element_3 0 (.R (Math|Color|BreakColor (LocalVariables|GetColor))) false)
        (Components|InstancedStaticMesh|SetCustomDataValue (Variables|Default|GetISM_BuildingBlocks) _array_element_3 1 (.G (Math|Color|BreakColor (LocalVariables|GetColor))) false)
        (Components|InstancedStaticMesh|SetCustomDataValue (Variables|Default|GetISM_BuildingBlocks) _array_element_3 2 (.B (Math|Color|BreakColor (LocalVariables|GetColor))) false)
        (Components|InstancedStaticMesh|SetCustomDataValue (Variables|Default|GetISM_BuildingBlocks) _array_element_3 3 1.0 false)
        (Components|InstancedStaticMesh|SetCustomDataValue (Variables|Default|GetISM_BuildingBlocks) _array_element_3 4 1.0 false)))))

(fn AddPCGBuildings
  (bind _cellsize (Variables|Default|GetCellSize))
  (bind _cellsize_2 (Variables|Default|GetCellSize))
  (bind _cellsize_3 (Variables|Default|GetCellSize))
  (for _array_element (Variables|Default|GetDistrictArray)
    (LocalVariables|SetDistrictType (.DistrictType (Utilities|Struct|BreakDistrictStruct _array_element)))
    (for _array_element_2 (.BlockCellArray (Utilities|Struct|BreakDistrictStruct _array_element))
      (LocalVariables|SetSizeX (.SizeX (Utilities|Struct|BreakBlockCellStruct _array_element_2)))
      (LocalVariables|SetSizeY (.SizeY (Utilities|Struct|BreakBlockCellStruct _array_element_2)))
      (if (Utilities|Array|IsNotEmpty (.BlockArray (Utilities|Struct|BreakBlockCellStruct _array_element_2)))
        (switch int (LocalVariables|GetDistrictType)
          (:1
            (Game|SpawnActorfromClass "/Game/Blueprint/Buildings/BP_BuildingPCG.BP_BuildingPCG_C" (Math|Transform|MakeTransform (+ (.location (.OutInstanceTransform (Components|InstancedStaticMesh|GetInstanceTransform (Variables|Default|GetInstancedGridMesh) (Utilities|Array|Get(acopy) (.BlockArray (Utilities|Struct|BreakBlockCellStruct _array_element_2))) true))) (Math|Vector|MakeVector (* (- (/ (Math|Conversions|ToFloat(Integer) (LocalVariables|GetSizeY)) (Math|Float|MakeLiteralFloat 2.0)) (Math|Float|MakeLiteralFloat 0.5)) _cellsize) (* (- (/ (Math|Conversions|ToFloat(Integer) (LocalVariables|GetSizeX)) (Math|Float|MakeLiteralFloat 2.0)) (Math|Float|MakeLiteralFloat 0.5)) _cellsize) 1e+01)) "0, 0, 0" "1.000000,1.000000,1.000000") "AlwaysSpawn" "MultiplyWithRoot" 0 (Math|Random|RandomIntegerinRange (Variables|Default|GetminHeightResidential) (Variables|Default|GetmaxHeightResidential)) (Math|Random|RandomInteger 10000) (LocalVariables|GetDistrictType) 0 0 0 false (- (LocalVariables|GetSizeX) 2) (- (LocalVariables|GetSizeY) 2) 0))
          (:2
            (Game|SpawnActorfromClass "/Game/Blueprint/Buildings/BP_BuildingPCG.BP_BuildingPCG_C" (Math|Transform|MakeTransform (+ (.location (.OutInstanceTransform (Components|InstancedStaticMesh|GetInstanceTransform (Variables|Default|GetInstancedGridMesh) (Utilities|Array|Get(acopy) (.BlockArray (Utilities|Struct|BreakBlockCellStruct _array_element_2))) true))) (Math|Vector|MakeVector (* (- (/ (Math|Conversions|ToFloat(Integer) (LocalVariables|GetSizeY)) (Math|Float|MakeLiteralFloat 2.0)) (Math|Float|MakeLiteralFloat 0.5)) _cellsize_2) (* (- (/ (Math|Conversions|ToFloat(Integer) (LocalVariables|GetSizeX)) (Math|Float|MakeLiteralFloat 2.0)) (Math|Float|MakeLiteralFloat 0.5)) _cellsize_2) 1e+01)) "0, 0, 0" "1.000000,1.000000,1.000000") "AlwaysSpawn" "MultiplyWithRoot" 0 (Math|Random|RandomIntegerinRange (Variables|Default|GetminHeightCommercial) (Variables|Default|GetmaxHeightCommercial)) (Math|Random|RandomInteger 10000) (LocalVariables|GetDistrictType) 0 0 0 false (LocalVariables|GetSizeX) (LocalVariables|GetSizeY) 0))
          (:3
            (Game|SpawnActorfromClass "/Game/Blueprint/Buildings/BP_BuildingPCG.BP_BuildingPCG_C" (Math|Transform|MakeTransform (+ (.location (.OutInstanceTransform (Components|InstancedStaticMesh|GetInstanceTransform (Variables|Default|GetInstancedGridMesh) (Utilities|Array|Get(acopy) (.BlockArray (Utilities|Struct|BreakBlockCellStruct _array_element_2))) true))) (Math|Vector|MakeVector (* (- (/ (Math|Conversions|ToFloat(Integer) (LocalVariables|GetSizeY)) (Math|Float|MakeLiteralFloat 2.0)) (Math|Float|MakeLiteralFloat 0.5)) _cellsize_3) (* (- (/ (Math|Conversions|ToFloat(Integer) (LocalVariables|GetSizeX)) (Math|Float|MakeLiteralFloat 2.0)) (Math|Float|MakeLiteralFloat 0.5)) _cellsize_3) 1e+01)) "0, 0, 0" "1.000000,1.000000,1.000000") "AlwaysSpawn" "MultiplyWithRoot" 0 (Math|Random|RandomIntegerinRange (Variables|Default|GetminHeightIndustrial) (Variables|Default|GetmaxHeightIndustrial)) (Math|Random|RandomInteger 10000) (LocalVariables|GetDistrictType) (Math|Random|RandomIntegerinRange 1 4) 0 0 false (LocalVariables|GetSizeX) (LocalVariables|GetSizeY) 0)))))))

(fn AddFoliage)

(fn GenerateMap
  (CallFunction|ClearMap)
  (Variables|Default|SetInSeed (Math|Random|RandomInteger 10000))
  (Variables|Default|SetTime (Math|DateTime|Now))
  (Utilities|FlowControl|Sequence
    (:then_0
      (Class|CACityLayout|Initialize)
      (Class|CACityLayout|Simulate)
      (Class|CACityLayout|TrimRoads)
      (Class|CACityLayout|AddRoadWidth)
      (Class|CACityLayout|VisualizeGrid))
    (:then_4
      (Class|CACityLayout|GetAllDistricts)
      (Class|CACityLayout|GetAllRoads)
      (Class|CACityLayout|SelectionSorttheRoad))
    (:then_8
      (Class|CACityLayout|InitializeLayerValues)
      (Class|CACityLayout|CalculateDistrictType)
      (Class|CACityLayout|FloorPlanAllDistricts))
    (:then_12
      (Class|CACityLayout|GetAllLargestRectanglesforDistricts))
    (:then_14
      (CallFunction|AddPCGBuildings))
    (:then_15
      (Class|CACityLayout|SetTreeLayerGridValues)
      (Class|CACityLayout|CalculateTileLayerGridValues)
      (Class|CACityLayout|CalculateRoadType))
    (:then_16
      (Development|PrintString (Utilities|String|Append "City Layout Generation Time :" (Utilities|String|ToString(Float) (Class|KismetMathLibrary|GetTotalMilliseconds (- (Math|DateTime|Now) (Variables|Default|GetTime)))) "ms")))))

(fn ClearMap
  (bind _outactors (Actor|GetAllActorsOfClass "/Game/Blueprint/Buildings/BP_BuildingPCG.BP_BuildingPCG_C"))
  (for _array_element _outactors
    (Actor|DestroyActor _array_element))
  (Components|InstancedStaticMesh|ClearInstances (Variables|Default|GetInstancedGridMesh))
  (Components|InstancedStaticMesh|ClearInstances (Variables|Default|GetISM_BuildingBlocks))
  (Components|InstancedStaticMesh|ClearInstances (Variables|Default|GetISMBush))
  (Components|InstancedStaticMesh|ClearInstances (Variables|Default|GetISMGrassV2))
  (Components|InstancedStaticMesh|ClearInstances (Variables|Default|GetISMGrass))
  (Components|InstancedStaticMesh|ClearInstances (Variables|Default|GetISMTreeV3))
  (Components|InstancedStaticMesh|ClearInstances (Variables|Default|GetISMTile))
  (Components|InstancedStaticMesh|ClearInstances (Variables|Default|GetISMTreeV2))
  (Components|InstancedStaticMesh|ClearInstances (Variables|Default|GetISMTree))
  (Components|InstancedStaticMesh|ClearInstances (Variables|Default|GetISMBlocks))
  (Utilities|Array|Clear (Variables|Default|GetDistrictArray)))

(fn ClearBuilding)