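; BPC_Spawnable is an actor component that shows whether its owner can be placed at its current location.
; On BeginPlay and on every begin or end overlap of the owner, it marks placement valid only when no actors overlap the owner.
; It then sets every material slot on all the owner's static meshes to the valid or invalid ploppable material to reflect that state.
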(event Custom|OverlapStatusChanged
  (params (OverlappedActor :type Actor%20Object%20Reference) (OtherActor :type Actor%20Object%20Reference))
  (CallFunction|UpdateState))

(event EventBeginPlay
  (bind _returnvalue (Components|GetOwner))
  (EventDispatchers|AssignOnActorBeginOverlap _returnvalue (delegate Custom|OverlapStatusChanged))
  (EventDispatchers|AssignOnActorEndOverlap _returnvalue (delegate Custom|OverlapStatusChanged))
  (CallFunction|UpdateState))

(fn UpdateState
  (Variables|Default|SetIsPlacementValid (== (Utilities|Array|Length (Collision|GetOverlappingActors (Components|GetOwner) "/Script/Engine.Actor" :!class /Script/Engine.Actor)) 0))
  (for _array_element (Actor|GetComponentsByClass (Components|GetOwner) "/Script/Engine.StaticMeshComponent")
    (for _index (range 0 (- (Utilities|Array|Length (Rendering|Material|GetMaterials _array_element)) 1))
      (if (Variables|Default|GetIsPlacementValid)
        (Rendering|Material|SetMaterial _array_element _index (Variables|Default|GetPloppableMaterial))
        (else
          (Rendering|Material|SetMaterial _array_element _index (Variables|Default|GetInvalidPloppableMaterial)))))))