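; Building actor that shows a tile-sized square area with border lines, hiding both meshes on BeginPlay if already placed.
; The construction script builds border and fill as procedural meshes, rotating only the border mesh by 45 degrees.
; CreateLine generates centered quads for both, with the fill being one line as thick as the tile.
; Each mesh gets a dynamic M_Grid material with its own color and opacity.
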(event EventBeginPlay
  (|CallParentFunction)
  (if (Variables|Default|GetIsPlaced)
    (Rendering|SetVisibility (Variables|Default|GetAreaProceduralMesh) false false)
    (Rendering|SetVisibility (Variables|Default|GetLinesProceduralMesh) false false)))

(event Collision|EventActorBeginOverlap
  (params (OtherActor :type Actor%20Object%20Reference)))

(event EventTick
  (params (DeltaSeconds :type Float%20%28single-precision%29)))

(fn ConstructionScript
  (bind _tilesize (Variables|Default|GetTileSize))
  (bind _returnvalue (/ _tilesize 2.0))
  (|CallParentFunction)
  (bind _materialinstance (CallFunction|CreateMaterialInstance (LocalVariables|GetLineColor) (LocalVariables|GetLineOpacity)))
  (Variables|Default|SetLinesMaterial _materialinstance)
  (bind _materialinstance_2 (CallFunction|CreateMaterialInstance (LocalVariables|GetAreaColor) (LocalVariables|GetAreaOpacity)))
  (LocalVariables|SetAreaMaterial _materialinstance_2)
  (Utilities|FlowControl|Sequence
    (:then_0
      ;[0.15 0.15 0.15 0.5] Create Horizontal Lines Geometry
      (for _index (range 0 1)
        (LocalVariables|SetLineStart (* _index (Variables|Default|GetTileSize)))
        (LocalVariables|SetLineEnd (Variables|Default|GetTileSize))
        (CallFunction|CreateLine (Math|Vector|MakeVector (LocalVariables|GetLineStart) 0.0 0.0) (Math|Vector|MakeVector (LocalVariables|GetLineStart) (LocalVariables|GetLineEnd) 0.0) 1e+01 (LocalVariables|GetLineVertices) (LocalVariables|GetLineTriangles))))
    (:then_1
      ;[0.15 0.15 0.15 0.5] Create Vertical Lines Geometry
      (for _index_2 (range 0 1)
        (LocalVariables|SetLineStart (* _index_2 (Variables|Default|GetTileSize)))
        (LocalVariables|SetLineEnd (Variables|Default|GetTileSize))
        (CallFunction|CreateLine (Math|Vector|MakeVector 0.0 (LocalVariables|GetLineStart) 0.0) (Math|Vector|MakeVector (LocalVariables|GetLineEnd) (LocalVariables|GetLineStart) 0.0) 1e+01 (LocalVariables|GetLineVertices) (LocalVariables|GetLineTriangles))))
    (:then_2
      (Class|ProceduralMeshComponent|CreateMeshSectionLinearColor (Variables|Default|GetLinesProceduralMesh) 0 (LocalVariables|GetLineVertices) (LocalVariables|GetLineTriangles) 0 0 0 0 0 0 0 false false)
      (Rendering|Material|SetMaterial (Variables|Default|GetLinesProceduralMesh) 0 (Variables|Default|GetLinesMaterial))
      (Transformation|SetWorldRotation (Variables|Default|GetLinesProceduralMesh) "0.000000,45.000000,0.000000" false false))
    (:then_3
      (CallFunction|CreateLine (Math|Vector|MakeVector 0.0 _returnvalue 0.0) (Math|Vector|MakeVector _tilesize _returnvalue 0.0) (Variables|Default|GetTileSize) (LocalVariables|GetSelectionVertices) (LocalVariables|GetSelectionTriangles))
      (Rendering|SetVisibility (Variables|Default|GetAreaProceduralMesh) true false)
      (Class|ProceduralMeshComponent|CreateMeshSectionLinearColor (Variables|Default|GetAreaProceduralMesh) 0 (LocalVariables|GetSelectionVertices) (LocalVariables|GetSelectionTriangles) 0 0 0 0 0 0 0 false false)
      (Rendering|Material|SetMaterial (Variables|Default|GetAreaProceduralMesh) 0 (LocalVariables|GetAreaMaterial)))))

(fn CreateLine
  (params (Start :type Vector) (End :type Vector) (Thickness :type Float%20%28double-precision%29) (Vertices :type Array%20of%20Vectors) (Triangles :type Array%20of%20Integers))
  (bind _tilesize (Variables|Default|GetTileSize))
  (bind _tilesize_2 (Variables|Default|GetTileSize))
  (bind _tilesize_3 (Variables|Default|GetTileSize))
  (bind _tilesize_4 (Variables|Default|GetTileSize))
  (bind _returnvalue (Utilities|Array|Length Vertices))
  (bind _returnvalue_2 (/ _tilesize_2 2.0))
  (bind _returnvalue_3 (/ _tilesize_4 2.0))
  (bind _returnvalue_4 (/ _tilesize 2.0))
  (bind _returnvalue_5 (/ _tilesize_3 2.0))
  (Utilities|FlowControl|Sequence
    (:then_0
      (LocalVariables|SetHalfThickness (/ Thickness 2.0))
      (LocalVariables|SetThicknessDirection (Math|Vector|CrossProduct (Math|Vector|Normalize (- End Start)) "0.000000,0.000000,1.000000")))
    (:then_1
      (Utilities|Array|AppendArray Triangles (Utilities|Array|MakeArray (+ _returnvalue 2) (+ _returnvalue 1) (+ _returnvalue 0) (+ _returnvalue 2) (+ _returnvalue 3) (+ _returnvalue 1)))
      (Utilities|Array|AppendArray Vertices (Utilities|Array|MakeArray (- (+ Start (* (LocalVariables|GetThicknessDirection) (LocalVariables|GetHalfThickness))) (Math|Vector|MakeVector _returnvalue_2 _returnvalue_2 0.0)) (- (+ End (* (LocalVariables|GetThicknessDirection) (LocalVariables|GetHalfThickness))) (Math|Vector|MakeVector _returnvalue_3 _returnvalue_3 0.0)) (- (- Start (* (LocalVariables|GetThicknessDirection) (LocalVariables|GetHalfThickness))) (Math|Vector|MakeVector _returnvalue_4 _returnvalue_4 0.0)) (- (- End (* (LocalVariables|GetThicknessDirection) (LocalVariables|GetHalfThickness))) (Math|Vector|MakeVector _returnvalue_5 _returnvalue_5 0.0)))))))

(fn CreateMaterialInstance
  (params (Color :type Linear%20Color%20Structure) (Opacity :type Float%20%28double-precision%29))
  (bind _returnvalue (Rendering|Material|CreateDynamicMaterialInstance "/Game/Material/M_Grid.M_Grid" "None" "None" :!class /Script/Engine.KismetMaterialLibrary))
  (Rendering|Material|SetVectorParameterValue _returnvalue "Color" Color :!class /Script/Engine.MaterialInstanceDynamic)
  (Rendering|Material|SetScalarParameterValue _returnvalue "Opacity" Opacity :!class /Script/Engine.MaterialInstanceDynamic)
  (return _returnvalue))