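; BP_PoliceStation is the police station building in a city builder, extending a parent building Blueprint.
; On BeginPlay, a placed station registers an effect layer with GM_CityBuilder using its type and placement coordinates.
; ClickActor shows or hides the area and line procedural meshes to match the clicked state.
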(event EventBeginPlay
  (|CallParentFunction)
  (if (Variables|Default|GetIsPlaced)
    (bind _asgm_city_builder (Utilities|Casting|CastToGM_CityBuilder (Game|GetGameMode)))
    (Default|AddBuildingEffectLayer _asgm_city_builder "PoliceStation" (Variables|Default|GetBuildingPlaceX) (Variables|Default|GetBuildingPlaceY))))

(event EventClickActor
  (params (IsClicked :type Boolean))
  (Rendering|SetVisibility (Variables|Default|GetAreaProceduralMesh) IsClicked false)
  (Rendering|SetVisibility (Variables|Default|GetLinesProceduralMesh) IsClicked false))

(fn ConstructionScript
  (|CallParentFunction))