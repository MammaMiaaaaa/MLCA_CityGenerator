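; BPC_ClickableComponent is an actor component that gives its owner click-toggle and hover feedback on a static mesh.
; On BeginPlay it binds the owner's click event, plus cursor-over events if a StaticMeshComponent is found.
; Each click flips IsClicked and swaps material slot 0 between BackgroundMaterial and ArrowMaterial.
; Hovering toggles custom depth rendering and its stencil value; disconnected overlay-material and custom-depth nodes remain unused.
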(event Custom|OnClicked_Event
  (params (TouchedActor :type Actor%20Object%20Reference) (ButtonPressed :type Key%20Structure :default "None"))
  (bind _staticmeshref (Variables|Default|GetStaticMeshRef))
  (bind _output_get (Variables|Default|SetIsClicked (not (Variables|Default|GetIsClicked))))
  (Utilities|IsValid (Variables|Default|GetStaticMeshRef)
    (:Is%20Valid
      (if _output_get
        (Rendering|Material|SetMaterial _staticmeshref 0 "/Engine/EngineMeshes/BackgroundMaterial.BackgroundMaterial")
        (else
          (Rendering|Material|SetMaterial _staticmeshref 0 "/Engine/VREditor/UI/ArrowMaterial.ArrowMaterial"))))))

(event Custom|OnBeginCursorOver_Event
  (params (TouchedActor :type Actor%20Object%20Reference))
  (bind _staticmeshref (Variables|Default|GetStaticMeshRef))
  (Rendering|SetRenderCustomDepth _staticmeshref true)
  (Rendering|SetCustomDepthStencilValue _staticmeshref 2))

(event Custom|OnEndCursorOver_Event
  (params (TouchedActor :type Actor%20Object%20Reference))
  (bind _staticmeshref (Variables|Default|GetStaticMeshRef))
  (Rendering|SetRenderCustomDepth _staticmeshref false)
  (Rendering|SetCustomDepthStencilValue _staticmeshref 0))

(event EventBeginPlay
  (bind _returnvalue (Components|GetOwner))
  (bind _returnvalue_2 (Actor|GetComponentbyClass _returnvalue "/Script/Engine.StaticMeshComponent"))
  (EventDispatchers|AssignOnClicked _returnvalue (delegate Custom|OnClicked_Event))
  (Utilities|IsValid _returnvalue_2
    (:Is%20Valid
      (Variables|Default|SetStaticMeshRef _returnvalue_2)
      (EventDispatchers|AssignOnBeginCursorOver _returnvalue (delegate Custom|OnBeginCursorOver_Event))
      (EventDispatchers|AssignOnEndCursorOver _returnvalue (delegate Custom|OnEndCursorOver_Event)))))