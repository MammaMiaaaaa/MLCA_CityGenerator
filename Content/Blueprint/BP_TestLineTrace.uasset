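; Test actor that rebuilds a 25x25 occupancy map of the area from its location once a second on a looping timer.
; Border cells are marked as walls, while inner cells box-trace vertically on Visibility and store the hit actor's name.
; Hit classes (building, cat, mouse, city layout) become integer codes in MappingArray, with other results adding no code.
; Each pass prints its generation time.
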(event Custom|LineTrace
  (bind _returnvalue (Transformation|GetActorLocation))
  (Utilities|Array|Clear (Variables|Default|GetLineTraceActor))
  (Utilities|Array|Clear (Variables|Default|GetMappingArray))
  (Variables|Default|SetTime (Math|DateTime|Now))
  (for _index (range 0 24)
    (for _index_2 (range 0 24)
      (if (Math|Boolean|ORBoolean (== _index_2 0) (== _index_2 24) (== _index 0) (== _index 24))
        (Utilities|Array|Add (Variables|Default|GetLineTraceActor) "Wall")
        (Utilities|Array|Add (Variables|Default|GetMappingArray) 1)
        (else
          (bind _outhit (Collision|BoxTraceByChannel (Math|Vector|MakeVector (+ (* _index 1600) (.x _returnvalue)) (+ (* _index_2 1600) (.y _returnvalue)) 1e+04) (Math|Vector|MakeVector (+ (* _index 1600) (.x _returnvalue)) (+ (* _index_2 1600) (.y _returnvalue)) 0.0) "500.000000,500.000000,500.000000" "0, 0, 0" "TraceTypeQuery1" false 0 "None" true "(R=1.000000,G=0.000000,B=0.000000,A=1.000000)" "(R=0.000000,G=1.000000,B=0.000000,A=1.000000)" 0.5))
          (Utilities|Array|Add (Variables|Default|GetLineTraceActor) (Utilities|GetDisplayName (.HitActor (Collision|BreakHitResult _outhit))))
          (if (== (Utilities|GetClass (.HitActor (Collision|BreakHitResult _outhit))) "/Game/Blueprint/Buildings/BP_BuildingPCG.BP_BuildingPCG_C")
            (Utilities|Array|Add (Variables|Default|GetMappingArray) 4)
            (elif (== (Utilities|GetClass (.HitActor (Collision|BreakHitResult _outhit))) "/Game/Blueprint/BP_Cat.BP_Cat_C")
              (Utilities|Array|Add (Variables|Default|GetMappingArray) 3)
              (elif (== (Utilities|GetClass (.HitActor (Collision|BreakHitResult _outhit))) "/Game/Blueprint/BP_Mouse.BP_Mouse_C")
                (Utilities|Array|Add (Variables|Default|GetMappingArray) 2)
                (elif (== (Utilities|GetClass (.HitActor (Collision|BreakHitResult _outhit))) "/Game/Blueprint/CellularAutomata/BP_CA_CityLayout.BP_CA_CityLayout_C")
                  (Utilities|Array|Add (Variables|Default|GetMappingArray) 0)))))))))
  (Development|PrintString (Utilities|String|Append "Generate Time" (Utilities|String|ToString(Float) (Class|KismetMathLibrary|GetTotalMilliseconds (- (Math|DateTime|Now) (Variables|Default|GetTime)))) "ms") true true "(R=0.000000,G=0.660000,B=1.000000,A=1.000000)" 1.0))

(event EventBeginPlay
  (bind _returnvalue (Utilities|Time|SetTimerbyEvent (delegate Custom|LineTrace) 1.0 true))
  (Variables|Default|SetTimerHandler _returnvalue))

(fn ConstructionScript)